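; AI follower pawn that flies alongside the player as a wingman and fires projectiles, registering itself with the player on BeginPlay.
; Looping timers query the player's flight state, interpolating rotation and floating-movement velocity toward the nearer left or right slot, with periodically randomized offsets.
; Follow speed scales with player speed.
; UpdateShooting toggles a timer spawning projectiles from the arrow and tightens rotation tracking while firing.
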(event Custom|VelocityUpdateTick
  (bind _floatingpawnmovement (Variables|Default|GetFloatingPawnMovement))
  (bind (_queryvalid_ _rot _left _right _speed) (Class|BPIFollowerTalk|FlyingPlayerQuery(Message) (Variables|Base|GetPlayer)))
  (Utilities|FlowControl|Sequence
    (:then_0
      (Transformation|SetActorRotation (Math|Interpolation|RInterpTo (Transformation|GetActorRotation) _rot (Variables|Movement|GetVelocityUpdateTickRate) (Variables|Movement|GetRInterpSpeed))))
    (:then_1
      (Variables|/Script/Engine.MovementComponent|SetVelocity _floatingpawnmovement (Math|Interpolation|VInterpTo (Variables|/Script/Engine.MovementComponent|GetVelocity _floatingpawnmovement) (* (Math|Vector|Normalize (- (+ (select (CallFunction|GetLR _left _right) _right _left) (Variables|RandomOffset|GetRandomOffset)) (Transformation|GetActorLocation))) (Math|Float|SelectFloat 1e+02 (+ (* _speed 0.9) 1.5e+02) (< (+ (* _speed 0.9) 1.5e+02) 2e+02))) (Variables|Movement|GetVelocityUpdateTickRate) (Variables|Movement|GetVinterpSpeed))))))

(event Custom|Generate%20Random%20Offset%20Tick
  (Variables|RandomOffset|SetRandomOffset (CallFunction|GenerateRandomOffset)))

(event Custom|Shoot%20Tick
  (bind _arrow (Variables|Default|GetArrow))
  (bind _returnvalue (Transformation|GetWorldTransform _arrow))
  (Game|SpawnActorfromClass "/Game/PsiCorps_Galactic/Blueprints/Projectiles/BP_CharacterProjectile.BP_CharacterProjectile_C" (Math|Transform|MakeTransform (.location _returnvalue) (.rotation _returnvalue) "1.000000,1.000000,1.000000") "Undefined" "MultiplyWithRoot" 0 4e+03 0.1 "/Game/Materials/MI_YellowEmissive.MI_YellowEmissive" 3.0 4.0 (Utilities|Array|MakeArray self (Variables|Base|GetPlayer)) 25.0 0))

(event EventBeginPlay
  (bind _output_get (Variables|Base|SetPlayer (Game|GetPlayerCharacter 0)))
  (Utilities|IsValid _output_get
    (:Is%20Valid
      (Class|BPIFollowerTalk|AddFollower(Message) _output_get self)
      (bind _returnvalue (Utilities|Time|SetTimerbyEvent (delegate Custom|Generate%20Random%20Offset%20Tick) (Variables|RandomOffset|GetRandomOffsetTickRate) true))
      (Variables|RandomOffset|SetRandomOffsetTimer _returnvalue)
      (bind _returnvalue_2 (Utilities|Time|SetTimerbyEvent (delegate Custom|VelocityUpdateTick) (Variables|Movement|GetVelocityUpdateTickRate) true))
      (Variables|Movement|SetVelocityUpdateTimer _returnvalue_2))))

(event EventUpdateShooting
  (params (StartShooting? :type Boolean))
  (if StartShooting?
    (bind _returnvalue (Utilities|Time|SetTimerbyEvent (delegate Custom|Shoot%20Tick) (Variables|Shooting|GetShootTickrate) true))
    (Variables|Default|SetShootTimer _returnvalue)
    (Variables|Movement|SetRInterpSpeed 2e+01)
    (else
      (Utilities|Time|ClearandInvalidateTimerbyHandle (Variables|Default|GetShootTimer))
      (Variables|Movement|SetRInterpSpeed 2.0))))

(event EventAddFollower
  (params (New%20Actor :type Actor%20Object%20Reference)))

(fn ConstructionScript)

(fn GenerateRandomOffset
  (bind _randomoffsetminmax (Variables|RandomOffset|GetRandomOffsetMinMax))
  (return (Math|Vector|MakeVector (Math|Random|RandomFloatinRange (* -1 (.x _randomoffsetminmax)) (.x _randomoffsetminmax)) (Math|Random|RandomFloatinRange (* -1 (.y _randomoffsetminmax)) (.y _randomoffsetminmax)) (Math|Random|RandomFloatinRange (* -1 (.z _randomoffsetminmax)) (.z _randomoffsetminmax)))))

(fn GetLR
  (params (Left :type Vector) (Right :type Vector))
  (bind _returnvalue (Transformation|GetActorLocation))
  (return (> (Math|Vector|VectorLength (- _returnvalue Left)) (Math|Vector|VectorLength (- _returnvalue Right)))))

(fn FlyingPlayerQuery
  (return false "0, 0, 0" "0, 0, 0" "0, 0, 0" 0.0))