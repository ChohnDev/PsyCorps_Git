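; Base projectile actor that moves with ProjectileMovement and damages the first world or pawn object it hits.
; A looping timer runs sphere traces from the previous location to half a trace interval ahead of the current one, covering the gaps between checks.
; A hit applies damage and destroys the projectile.
; The construction script applies lifespan, speed, gravity and cylinder material from variables.
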(event Custom|Tick
  (bind (_outhit _returnvalue) (Collision|SphereTraceForObjects (Variables|Default|GetPreviousLocation) (+ (Transformation|GetActorLocation) (* (Transformation|GetActorForwardVector) (* (Math|Vector|VectorLength (Variables|/Script/Engine.MovementComponent|GetVelocity (Variables|Default|GetProjectileMovement))) (Variables|Default|GetTraceTickrate) 0.5))) (Variables|Default|GetRadius) (Utilities|Array|MakeArray "ObjectTypeQuery1" "ObjectTypeQuery2" "ObjectTypeQuery3") false (Variables|Default|GetIgnoredActors) "None"))
  (if _returnvalue
    (Game|Damage|ApplyDamage (.HitActor (Collision|BreakHitResult _outhit)) (Variables|Default|GetDamage) 0 0)
    (Actor|DestroyActor)
    (else
      (Variables|Default|SetPreviousLocation (Transformation|GetActorLocation)))))

(event EventBeginPlay
  (bind _returnvalue (Utilities|Time|SetTimerbyEvent (delegate Custom|Tick) (Variables|Default|GetTraceTickrate) true))
  (Variables|Default|SetTraceTimer _returnvalue))

(fn ConstructionScript
  (bind _projectilemovement (Variables|Default|GetProjectileMovement))
  (bind _speed (Variables|Default|GetSpeed))
  (Variables|Default|SetPreviousLocation (Transformation|GetActorLocation))
  (Actor|SetLifeSpan (Variables|Default|GetLifespan))
  (Variables|/Script/Engine.ProjectileMovementComponent|SetInitialSpeed _projectilemovement _speed)
  (Variables|/Script/Engine.ProjectileMovementComponent|SetMaxSpeed _projectilemovement _speed)
  (Variables|/Script/Engine.ProjectileMovementComponent|SetProjectileGravityScale _projectilemovement (Variables|Default|GetGravity))
  (Rendering|Material|SetMaterial (Variables|Default|GetCylinder) 0 (Variables|Default|GetMaterial)))