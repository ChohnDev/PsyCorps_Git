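; Enemy spawner actor that populates an area with BP_Aggro enemies at level start.
; On BeginPlay it spawns SpawnAmount pawns through SpawnAIFromClass, each at a random point inside the Bound component's bounds.
; An unused SpawnCharacter function instead spawns one BP_Aggro at the world origin with random yaw, passing every BP_PatrolLocation in the level as its patrol points.
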(event EventBeginPlay
  (bind _bound (Variables|Default|GetBound))
  (bind (_origin _boxextent) (Collision|GetComponentBounds _bound))
  (for _index (range 1 (Variables|Default|GetSpawnAmount))
    (AI|SpawnAIFromClass "/Game/PsiCorps_Galactic/Blueprints/Enemy_AI/BP_Aggro.BP_Aggro_C" 0 (Math|Random|RandomPointinBoundingBox _origin _boxextent) "0, 0, 0" false 0)))

(fn ConstructionScript)

(fn SpawnCharacter
  (bind _outactors (Actor|GetAllActorsOfClass "/Game/PsiCorps_Galactic/Blueprints/Enemy_AI/BP_PatrolLocation.BP_PatrolLocation_C"))
  (Game|SpawnActorfromClass "/Game/PsiCorps_Galactic/Blueprints/Enemy_AI/BP_Aggro.BP_Aggro_C" (Math|Transform|MakeTransform "0, 0, 0" (Math|Rotator|MakeRotator 0.0 0.0 (Math|Random|RandomFloat))) "AlwaysSpawn" "MultiplyWithRoot" 0 _outactors 0))