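; BP_Aggro is a flying enemy AI pawn that patrols, chases and shoots the player.
; Looping timers drive vision checks (dot-product cone plus line trace), movement and shooting, switched by a FlyingMode state.
; It cycles shuffled BP_PatrolLocation points, moving by FloatingPawnMovement with interpolated rotation.
; In Aggro it fires projectiles when facing the player; on losing sight it searches the last seen location, spinning before resuming patrol.
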(event Custom|MovementTick
  ;[1 1 1] Movement
  (switch Utilities|FlowControl|Switch|SwitchonE_AggroFlyingMode (Variables|Movement|GetFlyingMode)
    (:NewEnumerator0
      (CallFunction|PatrolMovement))
    (:NewEnumerator1
      (CallFunction|AggroMovement))
    (:NewEnumerator2
      (CallFunction|LFPMovement))))

(event Custom|CheckForPlayer
  ;[1 1 1] CheckForPlayer
  (bind (_location _foundplayer_) (CallFunction|TraceforPlayer))
  (if _foundplayer_
    (Variables|Aggro|SetLastSawPlayerLocation _location)
    (Variables|Movement|SetFlyingMode "NewEnumerator1")
    (else
      (switch Utilities|FlowControl|Switch|SwitchonE_AggroFlyingMode (Variables|Movement|GetFlyingMode)
        (:NewEnumerator1
          (Variables|Movement|SetFlyingMode "NewEnumerator2")
          (Variables|Aggro|SetLookingForPlayerCounter 0))))))

(event Custom|LFPMovement
  (if (> (Math|Vector|VectorLength (- (Transformation|GetActorLocation) (Variables|Aggro|GetLastSawPlayerLocation))) (Variables|Aggro|GetAggroAcceptanceRadius))
    (CallFunction|DoMovementTick true true (Variables|Aggro|GetLastSawPlayerLocation))
    (else
      (Variables|/Script/Engine.MovementComponent|SetVelocity (Variables|Default|GetFloatingPawnMovement) "0, 0, 0")
      (bind _result (Math|Integer|IncrementInt (Variables|Aggro|GetLookingForPlayerCounter))
        (:%20%20
          (if (> _result (Variables|Aggro|GetMaxLFP))
            (Variables|Movement|SetFlyingMode "NewEnumerator0")
            (else
              (Class|Actor|AddActorWorldRotation (Math|Rotator|MakeRotator 0.0 0.0 (/ 3.6e+02 (Math|Conversions|ToFloat(Integer) (Variables|Aggro|GetMaxLFP))))))))))))

(event Custom|PatrolMovement
  (bind _patrolindex (Variables|Patrol|GetPatrolIndex))
  (bind _patrolpoints (Variables|Patrol|GetPatrolPoints))
  (bind _output (Utilities|Array|Get(acopy) _patrolpoints _patrolindex))
  ;[1 1 1] Patrol
  (if (Variables|Patrol|GetCanPatrol)
    (if (< (Transformation|GetDistanceTo self _output) (Variables|Patrol|GetPatrolAcceptanceRadius))
      (CallFunction|GetnextPatrolLocation)
      (else
        (CallFunction|DoMovementTick true true (Transformation|GetActorLocation _output))))))

(event Custom|AggroMovement
  (if (> (Math|Vector|VectorLength (- (Transformation|GetActorLocation) (Variables|Aggro|GetLastSawPlayerLocation))) (Variables|Aggro|GetAggroAcceptanceRadius))
    (CallFunction|DoMovementTick true true (Variables|Aggro|GetLastSawPlayerLocation))
    (else
      (CallFunction|DoMovementTick false true (Variables|Aggro|GetLastSawPlayerLocation))
      (Variables|/Script/Engine.MovementComponent|SetVelocity (Variables|Default|GetFloatingPawnMovement) "0, 0, 0"))))

(event Custom|DoMovementTick
  (params (DoForwardMovement :type Boolean) (DoRotation :type Boolean) (Location :type Vector))
  (bind _aggrorinterpspeed (Variables|Aggro|GetAggroRinterpSpeed))
  (bind _aggromovespeed (Variables|Aggro|GetAggroMovespeed))
  ;[1 1 1] Movement
  (Utilities|FlowControl|Sequence
    (:then_0
      (if DoForwardMovement
        (Class|PawnMovementComponent|AddInputVector (Variables|Default|GetFloatingPawnMovement) (* (Transformation|GetActorForwardVector) (Utilities|Select :Index (Variables|Movement|GetFlyingMode) :NewEnumerator0 (Variables|Patrol|GetPatrolMovespeed) :NewEnumerator1 _aggromovespeed :NewEnumerator2 _aggromovespeed)) false)))
    (:then_1
      (if DoRotation
        (Transformation|SetActorRotation (Math|Interpolation|RInterpTo (Transformation|GetActorRotation) (Math|Conversions|RotationFromXVector (Math|Vector|Normalize (- Location (Transformation|GetActorLocation)))) (Variables|Movement|GetMovementTickRate) (Utilities|Select :Index (Variables|Movement|GetFlyingMode) :NewEnumerator0 (Variables|Aggro|GetPatrolRinterpSpeed) :NewEnumerator1 _aggrorinterpspeed :NewEnumerator2 _aggrorinterpspeed)))))))

(event Custom|ShootTick
  (CallFunction|ChecktoShoot))

(event Custom|CheckToShoot
  (bind _arrow (Variables|Default|GetArrow))
  (bind _returnvalue (Transformation|GetWorldTransform _arrow))
  (switch Utilities|FlowControl|Switch|SwitchonE_AggroFlyingMode (Variables|Movement|GetFlyingMode)
    (:NewEnumerator1
      (if (> (Math|Vector|DotProduct (Math|Vector|GetForwardVector (Variables|Default|GetArrow)) (Math|Vector|Normalize (- (Transformation|GetActorLocation (Game|GetPlayerCharacter 0)) (Transformation|GetActorLocation)))) (Variables|Shooting|GetShootDot))
        (Game|SpawnActorfromClass "/Game/PsiCorps_Galactic/Blueprints/Projectiles/BP_BaseProjectile.BP_BaseProjectile_C" (Math|Transform|MakeTransform (.location _returnvalue) (.rotation _returnvalue) "1.000000,1.000000,1.000000") "Undefined" "MultiplyWithRoot" 0 3.0 2e+03 0.1 "/Game/PsiCorps_Galactic/Materials/Red_Emissive.Red_Emissive" 2.0 (Utilities|Array|MakeArray self) 5.0 0)))))

(event EventBeginPlay
  (bind _outactors (Actor|GetAllActorsOfClass "/Game/PsiCorps_Galactic/Blueprints/Enemy_AI/BP_PatrolLocation.BP_PatrolLocation_C"))
  (bind _output_get (Variables|Patrol|SetPatrolPoints _outactors))
  (Utilities|Array|Shuffle _output_get)
  (CallFunction|CheckCanPatrol)
  ;[1 1 1] Movement
  (bind _returnvalue (Utilities|Time|SetTimerbyEvent (delegate Custom|MovementTick) (Variables|Movement|GetMovementTickRate) true))
  (Variables|Movement|SetMovementTimer _returnvalue)
  ;[1 1 1] CheckForPlayer
  (bind _returnvalue_2 (Utilities|Time|SetTimerbyEvent (delegate Custom|CheckForPlayer) (Variables|CheckforPlayer|GetCheckForPlayerTick) true))
  (Variables|CheckForPlayer|SetCheckForPlayerTimer _returnvalue_2)
  (bind _returnvalue_3 (Utilities|Time|SetTimerbyEvent (delegate Custom|ShootTick) (Variables|Shooting|GetShootTickRate) true))
  (Variables|Shooting|SetShootTimer _returnvalue_3))

(fn ConstructionScript)

(fn CheckCanPatrol
  (if (> (Utilities|Array|Length (Variables|Patrol|GetPatrolPoints)) 0)
    (for _array_element (Variables|Patrol|GetPatrolPoints)
      (Utilities|IsValid _array_element
        (:Is%20Not%20Valid
          (Math|Integer|IncrementInt (LocalVariables|GetInvalidIndexes)))))
    (Variables|Patrol|SetCanPatrol (not (== (LocalVariables|GetInvalidIndexes) (Utilities|Array|Length (Variables|Patrol|GetPatrolPoints)))))
    (else
      (Variables|Patrol|SetCanPatrol false))))

(fn GetnextPatrolLocation
  (bind _output_get (Variables|Patrol|SetPatrolIndex (Math|Integer|SelectInt 0 (+ (Variables|Patrol|GetPatrolIndex) 1) (== (+ (Variables|Patrol|GetPatrolIndex) 1) (Utilities|Array|Length (Variables|Patrol|GetPatrolPoints)))) :!label _label))
  (Utilities|IsValid (Utilities|Array|Get(acopy) (Variables|Patrol|GetPatrolPoints) _output_get)
    (:Is%20Not%20Valid
      (goto _label))))

(fn TraceforPlayer
  (bind _returnvalue (Game|GetPlayerCharacter 0))
  (bind _returnvalue_2 (Transformation|GetActorLocation))
  (bind _arrow (Variables|Default|GetArrow))
  (bind _returnvalue_3 (Transformation|GetActorLocation _returnvalue))
  (bind _returnvalue_4 (Transformation|GetWorldLocation _arrow))
  (bind _returnvalue_5 (- _returnvalue_3 _returnvalue_2))
  (bind _returnvalue_6 (Math|Vector|Normalize _returnvalue_5))
  (if (> (Math|Vector|DotProduct (Math|Vector|GetForwardVector (Variables|Default|GetArrow)) _returnvalue_6) (Variables|CheckforPlayer|GetFindPlayerDot))
    (bind (_outhit _returnvalue_7) (Collision|LineTraceForObjects _returnvalue_4 (+ _returnvalue_4 (* _returnvalue_6 (Variables|CheckforPlayer|GetPlayerTraceDistance))) (Utilities|Array|MakeArray "ObjectTypeQuery1" "ObjectTypeQuery2" "ObjectTypeQuery3" "ObjectTypeQuery4" "ObjectTypeQuery5" "ObjectTypeQuery6") false 0 (select (Variables|CheckforPlayer|GetTraceDebug) "ForDuration" "None")))
    (if _returnvalue_7
      (return (.ImpactPoint (Collision|BreakHitResult _outhit)) (== (Game|GetPlayerCharacter 0) (.HitActor (Collision|BreakHitResult _outhit))))
      (else
        (return "0, 0, 0" false)))
    (else
      (return "0, 0, 0" false))))